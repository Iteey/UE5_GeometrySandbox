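; BP_Turret is an automated turret that shoots homing bullets at sensed pawns tagged TurretTarget.
; On sighting, it snaps the cube's yaw toward the pawn with random jitter and runs a looping Fire timer for a one-second burst.
; Each shot line-traces forward, updates the homing target on a tagged hit, and spawns a TurretBullet on any hit at one of four arrow muzzles, chosen randomly from positions cached on Tick.
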(event OnSeePawn(PawnSensing)
  (params (Pawn :type Pawn%20Object%20Reference))
  (bind _cube (Variables|Default|GetCube))
  (if (Actor|ActorHasTag Pawn "TurretTarget")
    (Transformation|SetWorldRotation _cube (Math|Rotator|MakeRotator 9e+01 0.0 (+ (+ (.yaw (Math|Rotator|FindLookatRotation (Transformation|GetWorldLocation _cube) (Transformation|GetWorldLocation (Variables|/Script/Engine.Actor|GetRootComponent Pawn)))) (Class|KismetSystemLibrary|MakeLiteralInteger 180)) (Math|Random|RandomFloatinRange -2.0 6.0))) false false)
    (bind _returnvalue (Utilities|Time|SetTimerbyEvent (delegate Custom|Fire) 0.1 true))
    (Utilities|FlowControl|Delay 1.0)
    (Audio|PlaySound2D "/Game/Enviromanet/Turret/shotgun-reload-old_school-ra_the_sun_god-580332022.shotgun-reload-old_school-ra_the_sun_god-580332022" 1.0 1.0 0.0 0 0)
    (Utilities|Time|ClearandInvalidateTimerbyHandle _returnvalue)))

(event Custom|Fire
  (bind _arrow (Variables|Default|GetArrow))
  (bind _returnvalue (Transformation|GetWorldLocation _arrow))
  (bind _outhit (Collision|LineTraceByChannel _returnvalue (+ _returnvalue (* (Math|Vector|GetForwardVector _arrow) (Class|KismetSystemLibrary|MakeLiteralInteger 5000))) "TraceTypeQuery1" true 0 "None"))
  (Utilities|IsValid (.HitActor (Collision|BreakHitResult _outhit))
    (:Is%20Valid
      (if (Actor|ActorHasTag (.HitActor (Collision|BreakHitResult _outhit)) "TurretTarget")
        (bind _output_get (Variables|Default|SetAim (.HitComponent (Collision|BreakHitResult _outhit)))))
      (Audio|PlaySound2D "/Game/Enviromanet/Turret/uhodyaschee-vdal-eho-posle-pistoletnogo-vyistrela.uhodyaschee-vdal-eho-posle-pistoletnogo-vyistrela" 1.0 1.0 0.0 0 0)
      (bind _returnvalue_2 (Game|SpawnActorfromClass "/Game/Enviromanet/Turret/TurretBullet.TurretBullet_C" (Math|Transform|MakeTransform (.OutItem (Utilities|Array|Random (Variables|Default|GetLocation%20array))) (.rotation (Transformation|GetWorldTransform (Variables|Default|GetArrow))) "1.000000,1.000000,1.000000") "Undefined" "MultiplyWithRoot" 0 0))
      (Variables|/Script/Engine.ProjectileMovementComponent|SetHomingTargetComponent (Variables|/Game/Enviromanet/Turret/TurretBullet.TurretBullet_C|GetProjectileMovement _returnvalue_2) _output_get))))

(event EventBeginPlay)

(event Collision|EventActorBeginOverlap
  (params (OtherActor :type Actor%20Object%20Reference)))

(event EventTick
  (params (DeltaSeconds :type Float%20%28single-precision%29))
  (bind _location_array (Variables|Default|GetLocation%20array))
  (Utilities|Array|SetArrayElem _location_array 0 (Transformation|GetWorldLocation (Variables|Default|GetArrow)))
  (Utilities|Array|SetArrayElem _location_array 1 (Transformation|GetWorldLocation (Variables|Default|GetArrow1)))
  (Utilities|Array|SetArrayElem _location_array 2 (Transformation|GetWorldLocation (Variables|Default|GetArrow2)))
  (Utilities|Array|SetArrayElem _location_array 3 (Transformation|GetWorldLocation (Variables|Default|GetArrow3))))

(fn ConstructionScript)