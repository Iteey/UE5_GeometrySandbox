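; Rocket-style projectile Blueprint that supplies the sound and particle effects for flight and impact.
; BeginPlay spawns a rocket sound at the spawn location and stores it in SoundRef, which is not used again here.
; Tick spawns a small P_Explosion emitter every frame as a trail.
; Hit plays a large version of the same emitter with an explosion sound; movement, damage and destruction are not handled in these graphs.
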(event EventBeginPlay
  (bind _returnvalue (Audio|SpawnSoundatLocation "/Game/Weapons/raketa-zvuk-raketyi-27936.raketa-zvuk-raketyi-27936" (Transformation|GetActorLocation) "0, 0, 0" 1.0 1.0 0.0 0 0))
  (Variables|Default|SetSoundRef _returnvalue))

(event Collision|EventActorBeginOverlap
  (params (OtherActor :type Actor%20Object%20Reference)))

(event EventTick
  (params (DeltaSeconds :type Float%20%28single-precision%29))
  (Utilities|FlowControl|Sequence
    (:then_0
      (Effects|SpawnEmitteratLocation "/Game/StarterContent/Particles/P_Explosion.P_Explosion" (.location (Transformation|GetActorTransform)) "0, 0, 0" "0.500000,0.500000,0.500000"))))

(event Collision|EventHit
  (params (MyComp :type Primitive%20Component%20Object%20Reference) (Other :type Actor%20Object%20Reference) (OtherComp :type Primitive%20Component%20Object%20Reference) (bSelfMoved :type Boolean) (HitLocation :type Vector :default "0, 0, 0") (HitNormal :type Vector :default "0, 0, 0") (NormalImpulse :type Vector :default "0, 0, 0") (Hit :type Hit%20Result%20Structure%20%28by%20ref%29))
  (bind _returnvalue (Transformation|GetActorLocation))
  (Effects|SpawnEmitteratLocation "/Game/StarterContent/Particles/P_Explosion.P_Explosion" _returnvalue "0, 0, 0" "7.000000,7.000000,7.000000")
  (Audio|PlaySoundatLocation "/Game/StarterContent/Audio/Explosion01.Explosion01" _returnvalue "0, 0, 0" 1.0 1.0 0.0 0 0 0 0))

(fn ConstructionScript)

(fn NewFunction)