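; Base player character Blueprint that takes turret bullet hits and ragdolls on death.
; Capsule overlaps with a TurretBullet call that bullet's ApplyDamage on the character.
; Tick polls HealthComponent and, at health of one or below, calls OnDeathPhysic to enable mesh physics and disable capsule collision.
; The same branch spawns the Damage effect at the head socket, repeating every frame while health stays that low.
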(event OnComponentBeginOverlap(CapsuleComponent)
  (params (OverlappedComponent :type Primitive%20Component%20Object%20Reference) (OtherActor :type Actor%20Object%20Reference) (OtherComp :type Primitive%20Component%20Object%20Reference) (OtherBodyIndex :type Integer) (bFromSweep :type Boolean) (SweepResult :type Hit%20Result%20Structure%20%28by%20ref%29))
  (Utilities|IsValid OtherActor
    (:Is%20Valid
      (bind _asturret_bullet (Utilities|Casting|CastToTurretBullet OtherActor))
      (Default|ApplyDamage _asturret_bullet self))))

(event EventBeginPlay)

(event Collision|EventActorBeginOverlap
  (params (OtherActor :type Actor%20Object%20Reference)))

(event EventTick
  (params (DeltaSeconds :type Float%20%28single-precision%29))
  (if (<= (Class|STUHealthComponent|GetHealth (Variables|Default|GetHealthComponent)) 1.0)
    (CallFunction|OnDeathPhysic)
    (Niagara|SpawnSystematLocation "/Game/VFX/Damage.Damage" (Transformation|GetSocketLocation (Variables|Character|GetMesh) "b_headSocket"))))

(event EventTalk)

(fn ConstructionScript)

(fn OnDeathPhysic
  (Physics|SetSimulatePhysics (Variables|Character|GetMesh) (<= (Class|STUHealthComponent|GetHealth (Variables|Default|GetHealthComponent)) 1.0))
  (Collision|SetCollisionEnabled (Variables|Default|GetCapsuleComponent) "NoCollision"))