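; Destructible turret that spots pawns tagged TurretTarget through PawnSensing and shoots projectiles at them.
; On sighting, it yaws its cube toward the pawn with random spread and runs a one-second looping-timer burst.
; Each shot requires any line-trace hit, then spawns a bullet at a random muzzle arrow location, refreshed every Tick.
; Damage, bound in Tick, lowers Health until the turret explodes and is destroyed.
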(event OnSeePawn(PawnSensing)
  (params (Pawn :type Pawn%20Object%20Reference))
  (bind _cube (Variables|Default|GetCube))
  (if (Actor|ActorHasTag Pawn "TurretTarget")
    (Transformation|SetWorldRotation _cube (Math|Rotator|MakeRotator 9e+01 0.0 (+ (+ (.yaw (Math|Rotator|FindLookatRotation (Transformation|GetWorldLocation _cube) (Transformation|GetWorldLocation (Variables|/Script/Engine.Actor|GetRootComponent Pawn)))) (Class|KismetSystemLibrary|MakeLiteralInteger 180)) (Math|Random|RandomFloatinRange -2.0 6.0))) false false)
    (bind _returnvalue (Utilities|Time|SetTimerbyEvent (delegate Custom|Fire) 0.1 true))
    (Utilities|FlowControl|Delay 1.0)
    (Audio|PlaySound2D "/Game/Enviromanet/Turret/shotgun-reload-old_school-ra_the_sun_god-580332022.shotgun-reload-old_school-ra_the_sun_god-580332022" 1.0 1.0 0.0 0 0)
    (Utilities|Time|ClearandInvalidateTimerbyHandle _returnvalue)))

(event Custom|OnTakeAnyDamage_Event
  (params (DamagedActor :type Actor%20Object%20Reference) (Damage :type Float%20%28single-precision%29) (DamageType :type Damage%20Type%20Object%20Reference) (InstigatedBy :type Controller%20Object%20Reference) (DamageCauser :type Actor%20Object%20Reference))
  (Audio|PlaySound2D "/Game/Enviromanet/Turret/mixkit-heavy-sword-hit-2794.mixkit-heavy-sword-hit-2794" 0.5 1.0 0.0 0 0)
  (Development|PrintString (Utilities|String|ToString(Float) (- (Variables|Default|GetHealth) Damage)))
  (bind _output_get (Variables|Default|SetHealth (- (Variables|Default|GetHealth) Damage)))
  (if (<= _output_get 0.0)
    (Development|PrintString "BYE")
    (Audio|PlaySound2D "/Game/Enviromanet/Turret/mixkit-explosion-hit-1704.mixkit-explosion-hit-1704" 0.7 1.0 0.0 0 0)
    (Effects|SpawnEmitteratLocation "/Game/StarterContent/Particles/P_Explosion.P_Explosion" (Transformation|GetWorldLocation (Variables|Default|GetCube)) "0, 0, 0" "6.000000,6.000000,6.000000")
    (Actor|DestroyActor)))

(event Custom|Fire
  (bind _arrow (Variables|Default|GetArrow))
  (bind _returnvalue (Transformation|GetWorldLocation _arrow))
  (bind _outhit (Collision|LineTraceByChannel _returnvalue (+ _returnvalue (* (Math|Vector|GetForwardVector _arrow) (Class|KismetSystemLibrary|MakeLiteralInteger 5000))) "TraceTypeQuery1" true 0 "None"))
  (Utilities|IsValid (.HitActor (Collision|BreakHitResult _outhit))
    (:Is%20Valid
      (if (Actor|ActorHasTag (.HitActor (Collision|BreakHitResult _outhit)) "TurretTarget")
        _
        (else
          _))
      (Audio|PlaySound2D "/Game/Enviromanet/Turret/uhodyaschee-vdal-eho-posle-pistoletnogo-vyistrela.uhodyaschee-vdal-eho-posle-pistoletnogo-vyistrela" 0.2 1.0 0.0 0 0)
      (bind _returnvalue_2 (Game|SpawnActorfromClass "/Game/Enviromanet/Turret/TurretBullet.TurretBullet_C" (Math|Transform|MakeTransform (.OutItem (Utilities|Array|Random (Variables|Default|GetLocation%20array))) (.rotation (Transformation|GetWorldTransform (Variables|Default|GetArrow))) "1.000000,1.000000,1.000000") "Undefined" "MultiplyWithRoot" 0 0))
      (Variables|/Script/Engine.ProjectileMovementComponent|SetHomingTargetComponent (Variables|/Game/Enviromanet/Turret/TurretBullet.TurretBullet_C|GetProjectileMovement _returnvalue_2) 0))))

(event EventBeginPlay)

(event Collision|EventActorBeginOverlap
  (params (OtherActor :type Actor%20Object%20Reference)))

(event EventTick
  (params (DeltaSeconds :type Float%20%28single-precision%29))
  (bind _location_array (Variables|Default|GetLocation%20array))
  (Utilities|Array|SetArrayElem _location_array 0 (Transformation|GetWorldLocation (Variables|Default|GetArrow)))
  (Utilities|Array|SetArrayElem _location_array 1 (Transformation|GetWorldLocation (Variables|Default|GetArrow1)))
  (Utilities|Array|SetArrayElem _location_array 2 (Transformation|GetWorldLocation (Variables|Default|GetArrow2)))
  (Utilities|Array|SetArrayElem _location_array 3 (Transformation|GetWorldLocation (Variables|Default|GetArrow3)))
  (EventDispatchers|AssignOnTakeAnyDamage (delegate Custom|OnTakeAnyDamage_Event)))

(fn ConstructionScript)

(fn NewFunction)