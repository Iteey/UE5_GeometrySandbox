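; BP_STUProjectileJump is a projectile actor that trails explosion particles and bursts on impact.
; Every Tick spawns an explosion emitter at the actor's location to form the trail.
; On Hit it spawns an enlarged explosion and two overlapping smoke emitters, then destroys itself, with no damage or jump logic in these graphs.
; A DestroyComp helper destroys a given component but is not called by the graphs shown.
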(event EventBeginPlay)

(event Collision|EventActorBeginOverlap
  (params (OtherActor :type Actor%20Object%20Reference)))

(event EventTick
  (params (DeltaSeconds :type Float%20%28single-precision%29))
  (Effects|SpawnEmitteratLocation "/Game/StarterContent/Particles/P_Explosion.P_Explosion" (Transformation|GetActorLocation)))

(event Collision|EventHit
  (params (MyComp :type Primitive%20Component%20Object%20Reference) (Other :type Actor%20Object%20Reference) (OtherComp :type Primitive%20Component%20Object%20Reference) (bSelfMoved :type Boolean) (HitLocation :type Vector :default "0, 0, 0") (HitNormal :type Vector :default "0, 0, 0") (NormalImpulse :type Vector :default "0, 0, 0") (Hit :type Hit%20Result%20Structure%20%28by%20ref%29))
  (Variables|Default|SetActorHitLocation (Transformation|GetActorLocation))
  (Effects|SpawnEmitteratLocation "/Game/StarterContent/Particles/P_Explosion.P_Explosion" (Variables|Default|GetActorHitLocation) "0, 0, 0" "12.000000,12.000000,12.000000")
  (Effects|SpawnEmitteratLocation "/Game/StarterContent/Particles/P_Smoke.P_Smoke" (Variables|Default|GetActorHitLocation) "0, 0, 0" "6.000000,6.000000,6.000000")
  (Effects|SpawnEmitteratLocation "/Game/StarterContent/Particles/P_Smoke.P_Smoke" (Variables|Default|GetActorHitLocation) "0, 0, 0" "6.000000,6.000000,6.000000")
  (Actor|DestroyActor))

(fn ConstructionScript)

(fn DestroyComp
  (params (Target :type Actor%20Component%20Object%20Reference))
  (Components|DestroyComponent Target))